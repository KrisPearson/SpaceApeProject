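; AI controller for paper-character NPCs that runs the Patrol_BT behavior tree.
; On BeginPlay it sets up PatrolData_BB with placeholder patrol points, stores the first PlayerPaperCharacter_BP found as TargetActor, then starts the tree.
; Every Tick it overwrites both patrol points with random XY positions inside the controlled character's room bounds, taking Z from the minimum and maximum bounds respectively.
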(event `self.ReceiveBeginPlay`
  (bind _blackboardcomponent (`self.UseBlackboard` "/Game/AI/PatrolData_BB.PatrolData_BB"))
  (`BlackboardComponent.SetValueAsVector` _blackboardcomponent "PatrolPointOne" (0.0 0.0 0.0))
  (`BlackboardComponent.SetValueAsVector` _blackboardcomponent "PatrolPointTwo" (300.0 300.0 0.0))
  (bind _outactors (`GameplayStatics.GetAllActorsOfClass` "/Game/CharacterBlueprints/PlayerPaperCharacter_BP.PlayerPaperCharacter_BP_C"))
  (`BlackboardComponent.SetValueAsObject` _blackboardcomponent "TargetActor" (`|GetArrayItem` _outactors))
  (`self.RunBehaviorTree` "/Game/AI/Patrol_BT.Patrol_BT"))

(event `self.ReceiveTick`
  (params (DeltaSeconds :type "Float (single-precision)"))
  (bind _asbase_paper_character (cast `BasePaperCharacter` (`self.K2_GetPawn`)))
  (bind _returnvalue (`BasePaperCharacter.GetRoomMinBounds` _asbase_paper_character))
  (bind _returnvalue_2 (`BasePaperCharacter.GetRoomMaxBounds` _asbase_paper_character))
  (bind _returnvalue_3 (`KismetMathLibrary.RandomFloatInRange` (.x _returnvalue) (.x _returnvalue_2)))
  (bind _returnvalue_4 (`KismetMathLibrary.RandomFloatInRange` (.y _returnvalue) (.y _returnvalue_2)))
  (`BlackboardComponent.SetValueAsVector` (stale `self.ReceiveBeginPlay` _blackboardcomponent) "PatrolPointOne" (`KismetMathLibrary.MakeVector` _returnvalue_3 _returnvalue_4 (.z _returnvalue)))
  (`BlackboardComponent.SetValueAsVector` (stale `self.ReceiveBeginPlay` _blackboardcomponent) "PatrolPointTwo" (`KismetMathLibrary.MakeVector` _returnvalue_3 _returnvalue_4 (.z _returnvalue_2))))

(fn `UserConstructionScript`)