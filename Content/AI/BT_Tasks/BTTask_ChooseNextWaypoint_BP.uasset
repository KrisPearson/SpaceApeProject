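; Behavior tree task that picks new random patrol waypoints for a BasePaperCharacter within its room.
; On execute, FindWaypoints reads the pawn's room min and max bounds and rolls random X/Y points at zero Z.
; It writes them to the PatrolPointOne and PatrolPointTwo blackboard keys, then the task finishes successfully.
; Points are purely random within the bounds, with no navigation or reachability check.
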(event `self.ReceiveExecuteAI`
  (params (OwnerController :type "AIController Object Reference") (ControlledPawn :type "Pawn Object Reference"))
  (`self.FindWaypoints` OwnerController ControlledPawn)
  (`self.FinishExecute` true))

(fn `FindWaypoints`
  (params (Blackboard :type "AIController Object Reference") (object :type "Actor Object Reference"))
  (bind _blackboard (`AIController.Blackboard` Blackboard))
  (bind _asbase_paper_character (cast `BasePaperCharacter` object))
  (bind _returnvalue (`BasePaperCharacter.GetRoomMinBounds` _asbase_paper_character))
  (bind _returnvalue_2 (`BasePaperCharacter.GetRoomMaxBounds` _asbase_paper_character))
  (bind _x (.x (`KismetMathLibrary.MakeVector` (`KismetMathLibrary.RandomFloatInRange` (.x _returnvalue) (.x _returnvalue_2)) (`KismetMathLibrary.RandomFloatInRange` (.y _returnvalue) (.y _returnvalue_2)))))
  (bind _y (.y (`KismetMathLibrary.MakeVector` (`KismetMathLibrary.RandomFloatInRange` (.x _returnvalue) (.x _returnvalue_2)) (`KismetMathLibrary.RandomFloatInRange` (.y _returnvalue) (.y _returnvalue_2)))))
  (`BlackboardComponent.SetValueAsVector` _blackboard "PatrolPointOne" (`KismetMathLibrary.MakeVector` _x _y))
  (`BlackboardComponent.SetValueAsVector` _blackboard "PatrolPointTwo" (`KismetMathLibrary.MakeVector` _x _y)))